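; First-person player character with walk, sprint, crouch, camera-shake head bob and physics object carrying and throwing.
; BeginPlay adds the Enhanced Input mapping and two test widgets.
; Tick line-traces from the camera for grabbable objects, moves the PhysicsHandle target ahead of the view while holding, and triggers state-based shakes, skipped when holding in observe mode.
; Crouch changes walk speed and lerps camera height with timelines, without resizing the capsule.
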(event Custom|Character_Headbops
  (bind _returnvalue (Transformation|GetVelocity))
  (bind _returnvalue_2 (Math|Vector|VectorLength _returnvalue))
  ;[1 1 1] Specific Headbops for Character State
  (if (and (> _returnvalue_2 0.0) (Character|CanJump))
    (if (< _returnvalue_2 4e+02)
      (Game|Feedback|ClientStartCameraShake (Game|GetPlayerController 0) "/Game/Kagami/GameFramework/Core/Character/Headbops/Walk.Walk_C" 1.0 "CameraLocal" "0, 0, 0")
      (else
        (Game|Feedback|ClientStartCameraShake (Game|GetPlayerController 0) "/Game/Kagami/GameFramework/Core/Character/Headbops/Sprint.Sprint_C" 1.0 "CameraLocal" "0, 0, 0")))
    (else
      (Game|Feedback|ClientStartCameraShake (Game|GetPlayerController 0) "/Game/Kagami/GameFramework/Core/Character/Headbops/Idle.Idle_C" 1.0 "CameraLocal" "0, 0, 0"))))

(event Custom|Uncrouch
  (bind _camera (Variables|Default|GetCamera))
  (bind _camera_2 (Variables|Default|GetCamera))
  (bind _returnvalue (Transformation|GetWorldLocation _camera))
  (bind _returnvalue_2 (Transformation|GetWorldLocation _camera_2))
  ;[1 1 1] Main Character Movement
  ;;[1 1 1] Crouching
  (Variables|Default|SetIsCrouching false)
  (Variables|/Script/Engine.CharacterMovementComponent|SetMaxWalkSpeed (Variables|Character|GetCharacterMovement) (Variables|Default|GetSpeed_Walking))
  (Variables|Default|SetNormalHalfHeight (+ (.z _returnvalue) 8e+01))
  (Variables|Default|SetCrouchedHalfHeight (.z _returnvalue))
  (bind _newtrack_0 (Timeline|Timeline PlayFromStart)
    (:Update
      (Transformation|SetWorldLocation _camera_2 (Math|Vector|MakeVector (.x _returnvalue_2) (.y _returnvalue_2) (Math|Float|Lerp (Variables|Default|GetCrouchedHalfHeight) (Variables|Default|GetNormalHalfHeight) _newtrack_0)) true true))))

(event Custom|Crouchh
  (bind _camera (Variables|Default|GetCamera))
  (bind _camera_2 (Variables|Default|GetCamera))
  (bind _returnvalue (Transformation|GetWorldLocation _camera_2))
  (bind _returnvalue_2 (Transformation|GetWorldLocation _camera))
  ;[1 1 1] Main Character Movement
  ;;[1 1 1] Crouching
  (Variables|Default|SetIsCrouching true)
  (Variables|/Script/Engine.CharacterMovementComponent|SetMaxWalkSpeed (Variables|Character|GetCharacterMovement) (Variables|Default|GetSpeed_Crouching%20))
  (Variables|Default|SetNormalHalfHeight (.z _returnvalue_2))
  (Variables|Default|SetCrouchedHalfHeight (- (.z _returnvalue_2) 8e+01))
  (bind _newtrack_0 (Timeline|CrouchChar PlayFromStart)
    (:Update
      (Transformation|SetWorldLocation _camera_2 (Math|Vector|MakeVector (.x _returnvalue) (.y _returnvalue) (Math|Float|Lerp (Variables|Default|GetNormalHalfHeight) (Variables|Default|GetCrouchedHalfHeight) _newtrack_0)) true true))))

(event Custom|RetrieveCamera)

(event Input|EnhancedActionEvents|EnhancedInputActionIA_Look
  (params (ActionValue :type Vector%202D%20Structure) (ElapsedSeconds :type Float%20%28double-precision%29) (TriggeredSeconds :type Float%20%28double-precision%29) (InputAction :type Input%20Action%20Object%20Reference :default "/Game/Kagami/GameFramework/Core/Character/Input/Navigation/IA_Look.IA_Look"))
  ;[1 1 1] Main Character Movement
  ;;[1 1 1] Look Up, Down, Left, Right
  (Pawn|Input|AddControllerYawInput (.x ActionValue))
  (Pawn|Input|AddControllerPitchInput (.y ActionValue)))

(event Input|EnhancedActionEvents|EnhancedInputActionIA_Move
  (params (ActionValue :type Vector%202D%20Structure) (ElapsedSeconds :type Float%20%28double-precision%29) (TriggeredSeconds :type Float%20%28double-precision%29) (InputAction :type Input%20Action%20Object%20Reference :default "/Game/Kagami/GameFramework/Core/Character/Input/Navigation/IA_Move.IA_Move"))
  (bind _returnvalue (Pawn|GetControlRotation :!class /Script/Engine.Pawn))
  ;[1 1 1] Main Character Movement
  ;;[1 1 1] Move Forward, Back, Left and Right
  (Pawn|Input|AddMovementInput (Math|Vector|GetRightVector (Math|Rotator|MakeRotator (.roll _returnvalue) 0.0 (.yaw _returnvalue))) (.x ActionValue) false)
  (Pawn|Input|AddMovementInput (Math|Vector|GetForwardVector (Math|Rotator|MakeRotator 0.0 0.0 (.yaw (Pawn|GetControlRotation :!class /Script/Engine.Pawn)))) (.y ActionValue) false))

(event Input|EnhancedActionEvents|EnhancedInputActionIA_Observe
  (params (ActionValue :type Boolean) (ElapsedSeconds :type Float%20%28double-precision%29) (TriggeredSeconds :type Float%20%28double-precision%29) (InputAction :type Input%20Action%20Object%20Reference :default "/Game/Kagami/GameFramework/Core/Character/Input/GameplayInput/IA_Observe.IA_Observe"))
  (if (Variables|Default|GetcanObserve)
    (Variables|Default|SetisDetecting true)))

(event Input|EnhancedActionEvents|EnhancedInputActionIA_Shift
  (params (ActionValue :type Boolean) (ElapsedSeconds :type Float%20%28double-precision%29) (TriggeredSeconds :type Float%20%28double-precision%29) (InputAction :type Input%20Action%20Object%20Reference :default "/Game/Kagami/GameFramework/Core/Character/Input/Navigation/IA_Shift.IA_Shift"))
  ;[1 1 1] Main Character Movement
  ;;[1 1 1] Sprint
  (:Triggered
    (if (Variables|Default|GetIsCrouching)
      (CallFunction|Uncrouch))
    (Variables|/Script/Engine.CharacterMovementComponent|SetMaxWalkSpeed (Variables|Character|GetCharacterMovement) (Variables|Default|GetSpeed_Running)))
  (:Completed
    (Variables|/Script/Engine.CharacterMovementComponent|SetMaxWalkSpeed (Variables|Character|GetCharacterMovement) (Variables|Default|GetSpeed_Walking))))

(event Input|EnhancedActionEvents|EnhancedInputActionIA_PickUp
  (params (ActionValue :type Boolean) (ElapsedSeconds :type Float%20%28double-precision%29) (TriggeredSeconds :type Float%20%28double-precision%29) (InputAction :type Input%20Action%20Object%20Reference :default "/Game/Kagami/GameFramework/Core/Character/Input/GameplayInput/IA_PickUp.IA_PickUp"))
  (bind _traceresult (Variables|Default|GetTraceResult))
  ;[1 1 1] Carry on Object if such is detected
  (:Started
    (if (Variables|Default|GetIsDetectingObject)
      (Physics|Components|PhysicsHandle|GrabComponentatLocationwithRotation (Variables|Default|GetPhysicsHandle) (.hitcomponent _traceresult) "None" (Transformation|GetWorldLocation (.hitcomponent _traceresult)) "0, 0, 0")
      (Variables|Default|SetIsHoldingObject true)))
  (:Completed
    (if (Variables|Default|GetIsHoldingObject)
      (Physics|Components|PhysicsHandle|ReleaseComponent (Variables|Default|GetPhysicsHandle))
      (Variables|Default|SetIsHoldingObject false))))

(event Input|EnhancedActionEvents|EnhancedInputActionIA_Throw
  (params (ActionValue :type Boolean) (ElapsedSeconds :type Float%20%28double-precision%29) (TriggeredSeconds :type Float%20%28double-precision%29) (InputAction :type Input%20Action%20Object%20Reference :default "/Game/Kagami/GameFramework/Core/Character/Input/GameplayInput/IA_Throw.IA_Throw"))
  (bind _physicshandle (Variables|Default|GetPhysicsHandle))
  ;[1 1 1] Throw Mechanic
  (if (Variables|Default|GetIsHoldingObject)
    (Variables|Default|SetTrownComponent (Class|PhysicsHandleComponent|GetGrabbedComponent _physicshandle))
    (Physics|Components|PhysicsHandle|ReleaseComponent _physicshandle)
    (Physics|SetPhysicsLinearVelocity (Variables|Default|GetTrownComponent) (* (Math|Vector|GetForwardVector (Variables|Default|GetCamera)) "2000.000000,2000.000000,500.000000") false "None")
    (Variables|Default|SetIsHoldingObject false)))

(event Input|EnhancedActionEvents|EnhancedInputActionIA_Crouch
  (params (ActionValue :type Boolean) (ElapsedSeconds :type Float%20%28double-precision%29) (TriggeredSeconds :type Float%20%28double-precision%29) (InputAction :type Input%20Action%20Object%20Reference :default "/Game/Kagami/GameFramework/Core/Character/Input/Navigation/IA_Crouch.IA_Crouch"))
  ;[1 1 1] Main Character Movement
  ;;[1 1 1] Crouching
  (:Started
    (if (Variables|Default|GetIsCrouching)
      (CallFunction|Uncrouch)
      (else
        (CallFunction|Crouchh)))))

(event EventBeginPlay
  ;[1 1 1] Input Mapping Set Up
  (bind _returnvalue (UserInterface|CreateWidget "/Game/Kagami/GameFramework/Core/Interactables/ObserveTest.ObserveTest_C"))
  (UserInterface|Viewport|AddtoViewport _returnvalue 0)
  (bind _returnvalue_2 (UserInterface|CreateWidget "/Game/Kagami/GameFramework/Core/Interactables/ClickTest.ClickTest_C"))
  (UserInterface|Viewport|AddtoViewport _returnvalue_2 0)
  (bind _asplayer_controller (Utilities|Casting|CastToPlayerController (Pawn|GetController)))
  (Utilities|IsValid (PlayerController|LocalPlayerSubsystems|GetEnhancedInputLocalPlayerSubsystem _asplayer_controller)
    (:Is%20Valid
      (Input|AddMappingContext (PlayerController|LocalPlayerSubsystems|GetEnhancedInputLocalPlayerSubsystem _asplayer_controller) "/Game/Kagami/GameFramework/Core/Character/Input/IMC_Kagami.IMC_Kagami" 0 "(bIgnoreAllPressedKeysUntilRelease=True,bForceImmediately=False,bNotifyUserSettings=False)"))))

(event EventTick
  (params (DeltaSeconds :type Float%20%28single-precision%29))
  (bind _camera (Variables|Default|GetCamera))
  ;[1 1 1] Add Headbop
  (Variables|Default|SetDelta%20Seconds DeltaSeconds)
  (CallFunction|TraceforInteractableObjects)
  (if (Variables|Default|GetIsHoldingObject)
    (Physics|Components|PhysicsHandle|SetTargetLocation (Variables|Default|GetPhysicsHandle) (+ (Transformation|GetWorldLocation _camera) (* (Math|Vector|GetForwardVector (Transformation|GetWorldRotation _camera)) 5e+02)))
    (if (not (Variables|Default|GetisDetecting))
      (CallFunction|CharacterHeadbops))
    (else
      (CallFunction|CharacterHeadbops))))

(fn ConstructionScript)

(fn TraceforInteractableObjects
  (bind _camera (Variables|Default|GetCamera))
  (bind _returnvalue (Transformation|GetWorldLocation _camera))
  (bind (_outhit _returnvalue_2) (Collision|LineTraceForObjects _returnvalue (+ _returnvalue (* (Math|Vector|GetForwardVector _camera) 5e+02)) (Variables|Default|GetObject%20Types) true 0 "ForDuration"))
  (if _returnvalue_2
    (Variables|Default|SetIsDetectingObject true)
    (Variables|Default|SetTraceResult _outhit)
    (else
      (Variables|Default|SetIsDetectingObject false))))