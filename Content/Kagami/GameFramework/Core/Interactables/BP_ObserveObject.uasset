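; BP_ObserveObject is an interactable trigger that stages a camera shot and enables observing when the main character enters its box.
; Entering fades in audio, cuts to one view target and immediately blends to a second, creating a camera move.
; The character is flagged as detecting until a delay ends.
; Any actor leaving the box clears the cached character's observe ability, as end overlap has no actor check.
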(event OnComponentBeginOverlap(Box)
  (params (OverlappedComponent :type Primitive%20Component%20Object%20Reference) (OtherActor :type Actor%20Object%20Reference) (OtherComp :type Primitive%20Component%20Object%20Reference) (OtherBodyIndex :type Integer) (bFromSweep :type Boolean) (SweepResult :type Hit%20Result%20Structure%20%28by%20ref%29))
  (bind _asbp_main_character (Utilities|Casting|CastToBP_MainCharacter OtherActor))
  (Variables|/Game/Kagami/GameFramework/Core/Character/BP_MainCharacter.BP_MainCharacter_C|SetisDetecting _asbp_main_character true)
  (bind _output_get (Variables|Default|SetAs%20BP%20Main%20Character _asbp_main_character))
  (Variables|Default|Setinitcamm (Variables|/Game/Kagami/GameFramework/Core/Character/BP_MainCharacter.BP_MainCharacter_C|GetCamera _output_get))
  (Variables|/Game/Kagami/GameFramework/Core/Character/BP_MainCharacter.BP_MainCharacter_C|SetcanObserve _output_get true)
  (Audio|Components|Audio|FadeIn (Variables|Default|GetAudio) 2.0 1.0 0.0 "Linear" :!class /Script/Engine.AudioComponent)
  (Game|Player|SetViewTargetwithBlend (Game|GetPlayerController 0) (Variables|Default|GetNewVar) 0.0 "VTBlend_Linear" 0.0 false)
  (Game|Player|SetViewTargetwithBlend (Game|GetPlayerController 0) (Variables|Default|GetNewVar_0) (Variables|Default|GetinitialCamera) "VTBlend_Linear" 0.0 false)
  (Utilities|FlowControl|Delay (Variables|Default|Getdelay))
  (Variables|/Game/Kagami/GameFramework/Core/Character/BP_MainCharacter.BP_MainCharacter_C|SetisDetecting _output_get false))

(event OnComponentEndOverlap(Box)
  (params (OverlappedComponent :type Primitive%20Component%20Object%20Reference) (OtherActor :type Actor%20Object%20Reference) (OtherComp :type Primitive%20Component%20Object%20Reference) (OtherBodyIndex :type Integer))
  (Variables|/Game/Kagami/GameFramework/Core/Character/BP_MainCharacter.BP_MainCharacter_C|SetcanObserve (Variables|Default|GetAs%20BP%20Main%20Character) false))

(event EventBeginPlay)

(event Collision|EventActorBeginOverlap
  (params (OtherActor :type Actor%20Object%20Reference)))

(event EventTick
  (params (DeltaSeconds :type Float%20%28single-precision%29)))

(fn ConstructionScript)